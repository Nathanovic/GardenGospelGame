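; BP_Plant is a sprite-based plant actor that grows over time while watered and healthy, then switches to its outgrown sprite.
; Tick advances growth only while BP_PlantWater reports healthy; GiveWater refills that component, and Die sets the dead sprite.
; BeginPlay registers the WG_Plant widget with HUD_Main and binds click and water-gone events.
; A sphere overlap shows the widget to the player once growth finishes.
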(event `Initialize`
  ;[1 1 1] Initialize
  (`|ExecutionSequence`
    (:`then_0`
      (`self.SetInitialPlantVisuals`))
    (:`then_2`
      (set `PlayerController.bShowMouseCursor` true (`GameplayStatics.GetPlayerController` 0)))))

(event `self.ReceiveBeginPlay`
  (bind _wg_plant (`self.WG_Plant`))
  (`|ExecutionSequence`
    (:`then_0`
      (`self.Initialize`))
    (:`then_1`
      (bind _ashud_main (cast `/Game/Blueprints/HUD_Main` (`PlayerController.GetHUD` (`GameplayStatics.GetPlayerController` 0))))
      (bind _output_get (set `self.HUDMain` _ashud_main))
      (bind _aswg_plant (cast `/Game/UI/WG_Plant` (`WidgetComponent.GetWidget` _wg_plant))
        (:`then`
          (bind _output_get_2 (set `self.As WG Plant` _aswg_plant))
          (`/Game/Blueprints/HUD_Main.InitializeWidget` _output_get _output_get_2 _wg_plant false))
        (:`CastFailed`
          (`KismetSystemLibrary.PrintString` "Cast to WG_Plant failed"))))
    (:`then_2`
      (if (`KismetSystemLibrary.IsValid` (`self.BP_Harvestable`))
        (bind _aswg_plant_2 (cast `/Game/UI/WG_Plant` (`WidgetComponent.GetUserWidgetObject` (`self.WG_Plant`))))
        (add `/Game/UI/WG_Plant.OnClickEvent` _aswg_plant_2 (`|CreateDelegate` (`self.BP_Harvestable`) :!event `Harvest`))
        (else
          (`KismetSystemLibrary.PrintString` "I don't have a harvest"))))
    (:`then_3`
      (bind _asbp_plant_water (cast `/Game/Blueprints/Plants/BP_PlantWater` (`self.BP_PlantWater`)))
      (add `/Game/Blueprints/Plants/BP_PlantWater.OnAllWaterGone` _asbp_plant_water (`|CreateDelegate` :!event `Die`)))))

(event `self.ReceiveTick`
  (params (DeltaSeconds :type "Float (single-precision)"))
  (`self.Grow` DeltaSeconds))

(event `self.Sphere.OnComponentBeginOverlap`
  (params (OverlappedComponent :type "PrimitiveComponent Object Reference") (OtherActor :type "Actor Object Reference") (OtherComp :type "PrimitiveComponent Object Reference") (OtherBodyIndex :type Integer) (bFromSweep :type Boolean) (SweepResult :type "HitResult Structure (by ref)"))
  (`KismetSystemLibrary.PrintString` (`KismetStringLibrary.Concat_StrStr` "This plant has water: " (`KismetStringLibrary.Conv_DoubleToString` (`/Game/Blueprints/Plants/BP_PlantWater.CurrentFill` (`self.BP_PlantWater`)))))
  (if (and (== OtherActor (`GameplayStatics.GetPlayerPawn` 0)) (`self.IsDoneGrowing`))
    (`Widget.SetVisibility` (`self.As WG Plant`) "Visible")))

(event `self.Sphere.OnComponentEndOverlap`
  (params (OverlappedComponent :type "PrimitiveComponent Object Reference") (OtherActor :type "Actor Object Reference") (OtherComp :type "PrimitiveComponent Object Reference") (OtherBodyIndex :type Integer))
  (if (== OtherActor (`GameplayStatics.GetPlayerPawn` 0))
    (if (and (== (stale `self.Sphere.OnComponentBeginOverlap` OtherActor) (`GameplayStatics.GetPlayerPawn` 0)) (`self.IsDoneGrowing`))
      (`Widget.SetVisibility` (`self.As WG Plant`) "Hidden"))))

(fn `Die`
  (`PaperSpriteComponent.SetSprite` (`self.Sprite`) (`self.DeadPlantSprite`)))

(fn `EvaluateHealth`)

(fn `FinishGrowing`
  (set `self.IsDoneGrowing` true)
  (`PaperSpriteComponent.SetSprite` (`self.Sprite`) (`self.OutgrownPlantSprite`)))

(fn `GiveWater`
  (set `self.Water` (+ (`self.Water`) 10))
  (`/Game/Blueprints/Plants/BP_PlantWater.GiveWater` (`self.BP_PlantWater`) 10.0))

(fn `Grow`
  (params (DeltaTime :type "Float (double-precision)"))
  (if (<= (`self.GrowthTime`) (`self.GrowthDuration`))
    (bind _ishealthy (`self.IsHealthy`))
    (if _ishealthy
      (bind _output_get (set `self.GrowthTime` (+ (`self.GrowthTime`) DeltaTime)))
      (if (>= _output_get (`self.GrowthDuration`))
        (`KismetSystemLibrary.PrintString` "Finish growing!")
        (`self.FinishGrowing`)))))

(fn `IsHealthy`
  (returns (IsHealthy :type Boolean))
  (bind _ishealthy (`/Game/Blueprints/Plants/BP_PlantWater.IsHealthy` (`self.BP_PlantWater`)))
  (return _ishealthy))

(fn `SetInitialPlantVisuals`
  (bind _startplantsprite (`self.StartPlantSprite`))
  ;[1 1 1] Set plant mesh
  (if (`KismetSystemLibrary.IsValid` _startplantsprite)
    (`PaperSpriteComponent.SetSprite` (`self.Sprite`) _startplantsprite)
    (else
      (`KismetSystemLibrary.PrintString` "No start sprite was added"))))

(fn `UserConstructionScript`)