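; BP_PlantWater tracks a plant's water level and whether it is high enough to count as healthy.
; Tick drains CurrentFill by DrinkSpeed over time, then sets AllWaterGone and fires OnAllWaterGone once it empties.
; GiveWater adds clamped water and prints a debug value, but never clears AllWaterGone, so draining stays stopped after emptying.
; IsHealthy compares the fill percentage against HealthyFillPercentage.
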(event `self.ReceiveBeginPlay`)

(event `self.ReceiveTick`
  (params (DeltaSeconds :type "Float (single-precision)"))
  (if (not (`self.AllWaterGone`))
    (bind _output_get (set `self.CurrentFill` (- (`self.CurrentFill`) (* DeltaSeconds (`self.DrinkSpeed`)))))
    (if (<= _output_get 0.0)
      (set `self.AllWaterGone` true)
      (`self.OnAllWaterGone`))))

(fn `GiveWater`
  (params (WaterAmount :type "Float (double-precision)"))
  (bind _returnvalue (`KismetMathLibrary.FClamp` (+ (`self.CurrentFill`) WaterAmount) 0.0 (`self.MaxFill`)))
  (set `self.CurrentFill` _returnvalue)
  (`KismetSystemLibrary.PrintString` (`KismetStringLibrary.Conv_DoubleToString` _returnvalue)))

(fn `IsHealthy`
  (returns (IsHealthy :type Boolean))
  (return (>= (* (/ (`self.CurrentFill`) (`self.MaxFill`)) 100.0) (`self.HealthyFillPercentage`))))