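; BP_Harvestable is a plant component that lets its owning actor be harvested for an item while its Amount lasts.
; Harvest reads the owner's world location and passes it with HarvestableItem to HarvestPlant on player 0's BP_PlayerState.
; It then decrements Amount and prints the remaining seed count, while GetPosition also prints the location for debugging.
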(event `self.ReceiveBeginPlay`)

(fn `GetPosition`
  (returns (NewParam :type "Vector Structure"))
  (bind _output_get (set `self.VectorOwner` (`Actor.K2_GetActorLocation` (`self.GetOwner`))))
  (`KismetSystemLibrary.PrintString` (`KismetStringLibrary.Conv_VectorToString` _output_get))
  (return _output_get))

(fn `Harvest`
  (bind _amount (`self.Amount`))
  (if (> (`self.Amount`) 0)
    (bind _newparam (`self.GetPosition`))
    (bind _asbp_player_state (cast `/Game/Blueprints/Player/BP_PlayerState` (`GameplayStatics.GetPlayerState` 0)))
    (`/Game/Blueprints/Player/BP_PlayerState.HarvestPlant` _asbp_player_state (`self.HarvestableItem`) _newparam)
    (bind _result (`/Engine/EditorBlueprintResources/StandardMacros.DecrementInt` _amount)
      (:`  `
        (set `self.Amount` _result)
        (`KismetSystemLibrary.PrintString` (`KismetStringLibrary.Concat_StrStr` (`KismetStringLibrary.Conv_IntToString` _amount) " seeds remaining"))))))