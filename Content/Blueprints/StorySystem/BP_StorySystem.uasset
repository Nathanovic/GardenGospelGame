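; Story system that tracks main story progress and delivers letters to the player through a mailbox in a garden game.
; On initialization it caches the main HUD, spawns BP_MailBox and sets its sprite if the first letter is ready.
; Opening mail shows the HUD mail widget and empties the sprite, while a flag array and last-read index determine unread letters.
; Only the first letter's text is defined, and ground-letter functions are empty stubs.
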(event `InitializeStory`
  ;[1 1 1] Trigger Start Story
  (bind _ashud_main (cast `/Game/Blueprints/HUD_Main` (`PlayerController.GetHUD` (`GameplayStatics.GetPlayerController` 0))))
  (set `self.As HUD Main` _ashud_main)
  (`self.StartStoryContext`))

(event `StartStoryContext`
  (bind _returnvalue (`|SpawnActorFromClass` "/Game/Blueprints/StorySystem/BP_MailBox.BP_MailBox_C" (`self.MailBoxTransform`) "Undefined" "MultiplyWithRoot" null null))
  (bind _output_get (set `self.MailBox` _returnvalue))
  (if (`|GetArrayItem` (`self.Letters ready to read`))
    (`PaperSpriteComponent.SetSprite` (`/Game/Blueprints/StorySystem/BP_MailBox.Sprite` _output_get) "/Game/Sprites/MailboxWithLetter_Sprite.MailboxWithLetter_Sprite")))

(fn `CreateMailOnGround`
  (params (LocationToSpawnLetter :type "Transform Structure") (Name :type String)))

(fn `DoWeHaveMailToRead?`
  (returns (`MailToRead?` :type Boolean))
  ;[1 1 1] find the first letter that is readable
  (for (_array_element _array_index) (`self.Letters ready to read`)
    (if _array_element
      (bind _output_get (set `self.ReadableLetterINT` _array_index))
      (break)))
  (if (> (`self.ReadableLetterINT`) (`self.ReadLetterINT`))
    (set `self.ReadLetterINT` (`self.ReadableLetterINT`))
    (`KismetArrayLibrary.Array_Set` (`self.Letters ready to read`) _output_get)
    (return true)
    (else
      (return false))))

(fn `GetStoryProgress`
  (returns (StoryProgress :type Integer))
  (return (`self.MainStoryProgress`)))

(fn `Ground Letter Opened`
  (params (LetterOnGround :type "/Game/Blueprints/StorySystem/BP_LetterGround Object Reference")))

(fn `MailOpened`
  (`/Game/Blueprints/HUD_Main.SpawnMailWidget` (`self.As HUD Main`))
  (`self.SetNoMail`))

(fn `SetNewMail`
  (`PaperSpriteComponent.SetSprite` (`/Game/Blueprints/StorySystem/BP_MailBox.Sprite` (`self.MailBox`)) "/Game/Sprites/MailboxWithLetter_Sprite.MailboxWithLetter_Sprite"))

(fn `SetNoMail`
  (`PaperSpriteComponent.SetSprite` (`/Game/Blueprints/StorySystem/BP_MailBox.Sprite` (`self.MailBox`)) "/Game/Sprites/MailboxEmpty_Sprite.MailboxEmpty_Sprite"))

(fn `SetStoryLettersWithLayout`
  (`KismetArrayLibrary.Array_AddUnique` (`self.Letters-MainTextArray`) (`|FormatText` "Dear PlayerName, Greetings! \n \nI wanted to reach out and inform you that I'll be temporarily absent, leaving you as the steward of this magnificent garden. I have complete faith in your ability to nurture and care for it with the same devotion as I do. " (`|FormatText` " \n") (`|FormatText` "PlayerName"))))

(fn `UpdateStoryProgression`
  (set `self.MainStoryProgress` (+ 1 (`self.MainStoryProgress`))))

(fn `UserConstructionScript`)