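; Grid-system plant holder that spawns, tracks and removes a single plant reference.
; SpawnPlant converts the given position to 3D, jitters X and Z by a random offset, spawns the prefab there and stores it if it is a BP_Plant, returning success.
; HasPlant checks that the stored reference is valid, and RemovePlant uses it before destroying the plant.
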(fn `CalculateSpawnPosition`
  (params (TargetPosition :type "Vector Structure"))
  (returns (SpawnPosition :type "Vector Structure"))
  (bind _randomspawnoffset (`self.RandomSpawnOffset`))
  (bind _returnvalue (* _randomspawnoffset -1.0))
  (bind _worldposition (`/Game/Blueprints/BP_FunctionLibrary.Get3DPosition` TargetPosition))
  (return (`KismetMathLibrary.MakeVector` (+ (.x _worldposition) (`KismetMathLibrary.RandomFloatInRange` _returnvalue _randomspawnoffset)) (.y _worldposition) (+ (.z _worldposition) (`KismetMathLibrary.RandomFloatInRange` _returnvalue _randomspawnoffset)))))

(fn `HasPlant`
  (returns (HasPlant :type Boolean))
  (return (`KismetSystemLibrary.IsValid` (`self.Plant`))))

(fn `RemovePlant`
  (bind _hasplant (`self.HasPlant`))
  (if _hasplant
    (`Actor.K2_DestroyActor` (`self.Plant`))))

(fn `SpawnPlant`
  (params (PlantPrefab :type "Actor Class Reference") (Position :type "Vector Structure"))
  (returns (Success :type Boolean))
  (bind _spawnposition (`self.CalculateSpawnPosition` Position))
  (bind _returnvalue (`|SpawnActorFromClass` PlantPrefab (`KismetMathLibrary.Conv_VectorToTransform` _spawnposition) "AlwaysSpawn" "MultiplyWithRoot" null null))
  (bind _asbp_plant (cast `/Game/Blueprints/Plants/BP_Plant` _returnvalue)
    (:`then`
      (set `self.Plant` _asbp_plant)
      (return true))
    (:`CastFailed`
      (return false))))