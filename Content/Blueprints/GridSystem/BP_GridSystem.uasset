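; BP_GridSystem spawns a grid of BP_Tile actors in the XZ plane on BeginPlay and keeps them in TileArray.
; SpawnXRow fills a row along X at GridSize spacing, converting each position with Get3DPosition and a Y offset.
; MoveToNextRow steps up in Z and repeats until YRowAmount rows exist.
; FinishedGridSpawning then passes the array to BP_playerController through GetTileArrray.
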(event `FinishedGridSpawning`
  ;[1 1 1] Final
  (bind _asbp_player_controller (cast `/Game/Blueprints/Player/BP_playerController` (`GameplayStatics.GetPlayerController` 0)))
  (bind _output_get (set `self.As BP Player Controller` _asbp_player_controller))
  (`/Game/Blueprints/Player/BP_playerController.GetTileArrray` _output_get (`self.TileArray`)))

(event `self.ReceiveBeginPlay`
  ;[1 1 1] Setup
  (`self.BuildGrid`))

(event `BuildGrid`
  ;[1 1 1] Setup
  (set `self.SpawnLocation` (0.0 0.0 0.0))
  (`self.Spawn X row`))

(event `Spawn X row`
  (bind (_spawnlocation_x _spawnlocation_y _spawnlocation_z) (`KismetMathLibrary.BreakVector` (`self.SpawnLocation`)))
  ;[1 1 1] spawn on X row full amount
  (set `self.Z_RowSpawned` (+ (`self.Z_RowSpawned`) 1))
  (while (< (`self.X_RowSpawned`) (`self.X_rowAmount`))
    (set `self.X_RowSpawned` (+ (`self.X_RowSpawned`) 1))
    (bind _worldposition (`/Game/Blueprints/BP_FunctionLibrary.Get3DPosition` (`self.SpawnLocation`) (`self.SpawnYOffset`)))
    (bind _returnvalue (`|SpawnActorFromClass` "/Game/Blueprints/GridSystem/BP_Tile.BP_Tile_C" (`KismetMathLibrary.Conv_VectorToTransform` _worldposition) "Undefined" "MultiplyWithRoot" null null))
    (bind _output_get (set `self.Tile` _returnvalue))
    (`KismetArrayLibrary.Array_Add` (`self.TileArray`) _output_get)
    (set `self.SpawnLocation` (`KismetMathLibrary.MakeVector` (+ _spawnlocation_x (`self.GridSize`)) _spawnlocation_y _spawnlocation_z)))
  (`self.move to next row`))

(event `move to next row`
  (bind (_spawnlocation_x _spawnlocation_y _spawnlocation_z) (`KismetMathLibrary.BreakVector` (`self.SpawnLocation`)))
  ;[1 1 1] move down on Z row
  (if (< (`self.Z_RowSpawned`) (`self.Y_rowAmount`))
    (set `self.SpawnLocation` (`KismetMathLibrary.MakeVector` 0.0 0.0 (+ _spawnlocation_z (`self.GridSize`))))
    (set `self.X_RowSpawned` 0)
    (`self.Spawn X row`)
    (else
      (`self.FinishedGridSpawning`))))

(fn `UserConstructionScript`)