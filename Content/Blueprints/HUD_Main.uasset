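; Main HUD actor for a planting game that shows per-tile plant UI and relays plant, water and harvest actions.
; It caches the BP_PlayerState on BeginPlay, then forwards each action to it using the tile's plant holder or harvestable item.
; A helper sets up widget components in screen space with game-and-UI input focus, while SpawnPlantWidget simply reveals the tile's existing PlantUI, leaving older widget-creation logic unused.
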(event `self.ReceiveBeginPlay`
  (bind _asbp_player_state (cast `/Game/Blueprints/Player/BP_PlayerState` (`GameplayStatics.GetPlayerState` 0)))
  (set `self.As BP Player State` _asbp_player_state))

(fn `Harvest`
  (params (tile :type "/Game/Blueprints/GridSystem/BP_Tile Object Reference"))
  (`/Game/Blueprints/Player/BP_PlayerState.HarvestPlant` (`self.As BP Player State`) (`/Game/Blueprints/Plants/BP_Harvestable.HarvestableItem` (`/Game/Blueprints/Plants/BP_Plant.BP_Harvestable` (`/Game/Blueprints/GridSystem/BP_PlantHolder.Plant` (`/Game/Blueprints/GridSystem/BP_Tile.BP_PlantHolder` tile))))))

(fn `InitializeWidget`
  (params (Widget :type "Widget Object Reference") (WidgetComp :type "WidgetComponent Object Reference") (StartVisible :type Boolean))
  (`WidgetComponent.SetWidgetSpace` WidgetComp "Screen")
  (`WidgetBlueprintLibrary.SetInputMode_GameAndUIEx` (`GameplayStatics.GetPlayerController` 0) Widget "DoNotLock" false)
  (if StartVisible
    (`Widget.SetVisibility` Widget "Visible")
    (else
      (`Widget.SetVisibility` Widget "Hidden"))))

(fn `Plant`
  (params (HoveredTile :type "/Game/Blueprints/GridSystem/BP_Tile Object Reference"))
  (`/Game/Blueprints/Player/BP_PlayerState.PlantSeed` (`self.As BP Player State`) (`/Game/Blueprints/GridSystem/BP_Tile.BP_PlantHolder` HoveredTile) (`self.K2_GetActorLocation` HoveredTile)))

(fn `SpawnPlantWidget`
  (params (`tile of plant` :type "/Game/Blueprints/GridSystem/BP_Tile Object Reference"))
  (`SceneComponent.SetVisibility` (`/Game/Blueprints/GridSystem/BP_Tile.PlantUI` `tile of plant`) true false))

(fn `UserConstructionScript`)

(fn `Water`
  (params (Tile :type "/Game/Blueprints/GridSystem/BP_Tile Object Reference"))
  (`/Game/Blueprints/Player/BP_PlayerState.GiveWater` (`self.As BP Player State`) (`/Game/Blueprints/GridSystem/BP_Tile.BP_PlantHolder` Tile)))