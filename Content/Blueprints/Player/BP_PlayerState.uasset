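; Player state that provides the player's farming actions: harvesting, planting seeds and watering plants.
; Harvesting adds one of the item to the BPInventory map.
; Planting has the given plant holder spawn the first inventory key's plant prefab without consuming it, and returns false when the inventory is empty.
; Watering passes a fixed amount to the water component of the holder's plant, if one exists.
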(fn `GiveWater`
  (params (PlantHolder :type "/Game/Blueprints/GridSystem/BP_PlantHolder Object Reference"))
  (bind _hasplant (`/Game/Blueprints/GridSystem/BP_PlantHolder.HasPlant` PlantHolder))
  (if _hasplant
    (`/Game/Blueprints/Plants/BP_PlantWater.GiveWater` (`/Game/Blueprints/Plants/BP_Plant.BP_PlantWater` (`/Game/Blueprints/GridSystem/BP_PlantHolder.Plant` PlantHolder)) 10.0)))

(fn `HarvestPlant`
  (params (Item :type "/Game/Blueprints/ObtainableItem Structure"))
  (`/Game/Blueprints/Player/BP_Inventory.AddItem` (`self.BP_Inventory`) Item 1))

(fn `PlantSeed`
  (params (PlantHolder :type "/Game/Blueprints/GridSystem/BP_PlantHolder Object Reference") (Position :type "Vector Structure"))
  (returns (Success :type Boolean))
  (locals (Items :type "Map of /Game/Blueprints/ObtainableItem Structure to Integer") (SeedToPlant :type "/Game/Blueprints/ObtainableItem Structure") (PlantSpawner :type "/Game/Blueprints/GridSystem/BP_PlantHolder Object Reference") (SpawnPosition :type "Vector Structure"))
  (bind _allitems (`/Game/Blueprints/Player/BP_Inventory.AllItems` (`self.BP_Inventory`)))
  (set `local.SpawnPosition` Position)
  (set `local.PlantSpawner` PlantHolder)
  (set `local.Items` _allitems)
  (bind _keys (`BlueprintMapLibrary.Map_Keys` _allitems))
  (if (> (`KismetArrayLibrary.Array_Length` _keys) 0)
    (bind _keys_2 (`BlueprintMapLibrary.Map_Keys` (`local.Items`)))
    (bind (_output_harvestable _output_name _output_rarity _output_sprite _output_plantprefab) (break `/Game/Blueprints/ObtainableItem` (`|GetArrayItem` _keys_2)))
    (`/Game/Blueprints/GridSystem/BP_PlantHolder.SpawnPlant` (`local.PlantSpawner`) _output_plantprefab (`local.SpawnPosition`))
    (`KismetSystemLibrary.PrintString` "Plant it!")
    (return true)
    (else
      (return false))))

(fn `UserConstructionScript`)