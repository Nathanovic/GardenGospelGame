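; BP_Inventory is a player inventory that tracks item quantities in the AllItems map, keyed by item.
; AddItem increments an existing entry or creates one, then prints the count and item name.
; RemoveItem passes a negated amount to AddItem for existing items, so entries are never deleted or clamped at zero, and prints a warning for missing ones.
; GetAmount returns the number of map entries rather than total quantity.
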(fn `AddItem`
  (params (Item :type "/Game/Blueprints/ObtainableItem Structure") (Amount :type Integer))
  (locals (MyItem :type "/Game/Blueprints/ObtainableItem Structure"))
  (bind (_myitem_harvestable _myitem_name) (break `/Game/Blueprints/ObtainableItem` (`local.MyItem`)))
  (bind _output_get (set `local.MyItem` Item))
  (bind (_value _returnvalue) (`BlueprintMapLibrary.Map_Find` (`self.AllItems`) _output_get))
  (if _returnvalue
    (`BlueprintMapLibrary.Map_Add` (`self.AllItems`) (`local.MyItem`) (+ _value Amount))
    (else
      (`BlueprintMapLibrary.Map_Add` (`self.AllItems`) (`local.MyItem`) Amount)))
  (`KismetSystemLibrary.PrintString` (`KismetStringLibrary.Concat_StrStr` (`KismetStringLibrary.Concat_StrStr` "You have " (`KismetStringLibrary.Conv_IntToString` (`BlueprintMapLibrary.Map_Find` (`self.AllItems`) (`local.MyItem`)))) _myitem_name)))

(fn `GetAmount`
  (returns (Amount :type Integer))
  (return (`BlueprintMapLibrary.Map_Length` (`self.AllItems`))))

(fn `RemoveItem`
  (params (Item :type "/Game/Blueprints/ObtainableItem Structure") (Amount :type Integer))
  (if (`.ReturnValue` (`BlueprintMapLibrary.Map_Find` (`self.AllItems`) Item))
    (`self.AddItem` Item (* Amount -1))
    (else
      (`KismetSystemLibrary.PrintString` "Trying to remove an item that doesn't exist in the inventory"))))