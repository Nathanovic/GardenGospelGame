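; Player controller that highlights the grid tile under the mouse and opens a planting UI on left click.
; While the UI is closed, a delayed Tick traces from the cursor and, on a "Tile"-tagged hit, picks the nearest actor in the supplied tile array.
; A single highlight actor, ignored by the trace, follows that tile.
; Clicking passes the tile to HUD_Main and sets OpenUI, pausing hover checks.
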(event `EnhancedInput|/Game/IA_LeftClick`
  (params (ActionValue :type Boolean) (ElapsedSeconds :type "Float (double-precision)") (TriggeredSeconds :type "Float (double-precision)") (InputAction :type "InputAction Object Reference" :default "/Game/IA_LeftClick.IA_LeftClick"))
  ;[0 0 0] UI
  ;;[1 1 1] check if we can spawn tile UI on left click
  (:`Started`
    (if (`self.HoveringTile?`)
      (`self.SpawnPlantUI`)
      (set `self.OpenUI?` true)
      (else
        (`KismetSystemLibrary.PrintString` "no valid tile")))))

(event `SpawnPlantUI`
  ;[0 0 0] UI
  ;;[1 1 1] spawn plant UI
  (bind _ashud_main (cast `/Game/Blueprints/HUD_Main` (`self.GetHUD`))
    (:`then`
      (`/Game/Blueprints/HUD_Main.SpawnPlantWidget` _ashud_main (`self.HoveredTile`)))
    (:`CastFailed`
      (`KismetSystemLibrary.PrintString` "cast failed"))))

(event `self.ReceiveTick`
  (params (DeltaSeconds :type "Float (single-precision)"))
  (bind _gridhighlight (`self.GridHighlight`))
  (bind (_worldlocation _worlddirection) (`self.DeprojectMousePositionToWorld` (`GameplayStatics.GetPlayerController` 0)))
  ;[0 0.2604 0.1865] check what tile we hover & spawn highlight
  ;;[1 1 1] check mouse location
  (if (not (`self.OpenUI?`))
    (`KismetSystemLibrary.Delay` 0.1)
    (bind (_outhit _returnvalue) (`KismetSystemLibrary.LineTraceSingle` _worldlocation (+ _worldlocation (* _worlddirection 5000.0)) "TraceTypeQuery1" false (`self.ActorsToIgnoreArray`) "None" true (struct :`R` 1.0 :`A` 1.0) (struct :`G` 1.0 :`A` 1.0) 3.0))
    (if _returnvalue
      (bind (_bblockinghit _binitialoverlap _time _distance _location _impactpoint _normal _impactnormal _physmat _hitactor) (`GameplayStatics.BreakHitResult` _outhit))
      (if (`self.ActorHasTag` _hitactor "Tile")
        (`self.GetTileHovered2` _location)
        (set `self.HoveringTile?` true)
        (else
          (`/Engine/EditorBlueprintResources/StandardMacros.IsValid` _gridhighlight
            (:`Is Valid`
              (`self.K2_DestroyActor` _gridhighlight)
              (set `self.HoveringTile?` false))))))))

(event `GetTileHovered2`
  (params (NewParam :type "Vector Structure"))
  (bind _output (`|GetArrayItem` (`self.TileArray`)))
  (bind _returnvalue (`self.K2_GetActorLocation` _output))
  (bind _returnvalue_2 (`SceneComponent.K2_GetComponentLocation` (`/Game/Blueprints/GridSystem/BP_Tile.DefaultSceneRoot` (`self.HoveredTile`))))
  ;[0 0.2604 0.1865] check what tile we hover & spawn highlight
  ;;[1 1 1] setting initial value based on first from array
  (set `self.ClosestPosition` _returnvalue)
  (set `self.HoveredTile` _output)
  (set `self.ClosestDistance` (`KismetMathLibrary.Vector_Distance` _returnvalue NewParam))
  ;;[1 1 1] comparing rest of the array, see what one is closer
  (for _array_element (`self.TileArray`)
    (bind _returnvalue_3 (`self.K2_GetActorLocation` _array_element))
    (bind _returnvalue_4 (`KismetMathLibrary.Vector_Distance` _returnvalue_3 NewParam))
    (if (< _returnvalue_4 (`self.ClosestDistance`))
      (set `self.ClosestPosition` _returnvalue_3)
      (set `self.ClosestDistance` _returnvalue_4)
      (set `self.HoveredTile` _array_element)))
  ;;;[1 1 1] set highlight on currently hovered object
  (`/Engine/EditorBlueprintResources/StandardMacros.IsValid` (`self.GridHighlight`)
    (:`Is Valid`
      (`self.K2_SetActorLocation` (`self.GridHighlight`) _returnvalue_2 false false))
    (:`Is Not Valid`
      (bind _returnvalue_5 (`|SpawnActorFromClass` "/Game/Blueprints/GridSystem/BP_GridHighlight.BP_GridHighlight_C" (`KismetMathLibrary.Conv_VectorToTransform` _returnvalue_2) "Undefined" "MultiplyWithRoot" null null))
      (set `self.GridHighlight` _returnvalue_5)
      (`KismetArrayLibrary.Array_Add` (`self.ActorsToIgnoreArray`) (`self.GridHighlight`)))))

(fn `GetHoveredTile`
  (returns (NewParam :type "/Game/Blueprints/GridSystem/BP_Tile Object Reference"))
  (bind _hoveredtile (`self.HoveredTile`))
  (`/Engine/EditorBlueprintResources/StandardMacros.IsValid` _hoveredtile
    (:`Is Valid`
      (return _hoveredtile))))

(fn `GetTileArrray`
  (params (Tiles :type "Array of /Game/Blueprints/GridSystem/BP_Tile Object Reference"))
  (set `self.TileArray` Tiles))

(fn `UserConstructionScript`)